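; Whitebox 4x3 door Blueprint for tile data, with a mesh that slides vertically.
; It records the mesh's world position at BeginPlay, then each Tick offsets Z by the smoothed slide value from GetSlideSmooth times DoorSize.Y, scaled by 100.
; The construction script runs the parent's logic, then applies a solid material to the mesh when the door is sealed.
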(event `self.ReceiveBeginPlay`
  (set `self.BaseDoorLocation` (`SceneComponent.K2_GetComponentLocation` (`self.DoorMesh`))))

(event `self.ReceiveTick`
  (params (DeltaSeconds :type "Float (single-precision)"))
  (bind (_basedoorlocation_x _basedoorlocation_y _basedoorlocation_z) (`KismetMathLibrary.BreakVector` (`self.BaseDoorLocation`)))
  (bind (_doorsize_x _doorsize_y) (break `IntPoint` (`self.DoorSize`)))
  (`SceneComponent.K2_SetWorldLocation` (`self.DoorMesh`) (`KismetMathLibrary.MakeVector` _basedoorlocation_x _basedoorlocation_y (+ _basedoorlocation_z (* (`self.GetSlideSmooth`) _doorsize_y 100))) false false))

(fn `UserConstructionScript`
  (`parent.UserConstructionScript`)
  (if (`self.bIsSealed`)
    (`PrimitiveComponent.SetMaterial` (`self.DoorMesh`) 0 "/Game/LevelPrototyping/Materials/M_Solid.M_Solid")))